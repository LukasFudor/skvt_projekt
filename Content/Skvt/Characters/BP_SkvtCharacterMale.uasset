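; Male player character Blueprint with Enhanced Input look, camera-yaw-relative movement, jump and toggled crouch on a spring-arm camera.
; Crouching changes jump velocity, nudges the boom's height through OffsetCameraZ, and plays or reverses a timeline driving arm length.
; OffsetCameraZ applies a single interpolation step per call, and the timeline's camera-height node is disconnected.
; The CanJumpInternal override permits jumping whenever the character is not falling, including while crouched.
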(event `EnhancedInput|/Game/Skvt/Characters/Input/Actions/IA_Look`
  (params (ActionValue :type "Vector2D Structure") (ElapsedSeconds :type "Float (double-precision)") (TriggeredSeconds :type "Float (double-precision)") (InputAction :type "InputAction Object Reference" :default "/Game/Skvt/Characters/Input/Actions/IA_Look.IA_Look"))
  (:`Triggered`
    (`self.AddControllerYawInput` ActionValue_X)
    (`self.AddControllerPitchInput` ActionValue_Y)))

(event `EnhancedInput|/Game/Skvt/Characters/Input/Actions/IA_Jump`
  (params (ActionValue :type Boolean) (ElapsedSeconds :type "Float (double-precision)") (TriggeredSeconds :type "Float (double-precision)") (InputAction :type "InputAction Object Reference" :default "/Game/Skvt/Characters/Input/Actions/IA_Jump.IA_Jump"))
  (:`Triggered`
    (`self.Jump`))
  (:`Completed`
    (`self.StopJumping`)))

(event `EnhancedInput|/Game/Skvt/Characters/Input/Actions/IA_Move`
  (params (ActionValue :type "Vector2D Structure") (ElapsedSeconds :type "Float (double-precision)") (TriggeredSeconds :type "Float (double-precision)") (InputAction :type "InputAction Object Reference" :default "/Game/Skvt/Characters/Input/Actions/IA_Move.IA_Move"))
  (bind (_returnvalue_roll _returnvalue_pitch _returnvalue_yaw) (`KismetMathLibrary.BreakRotator` (`self.GetControlRotation`)))
  (bind (_returnvalue_roll_2 _returnvalue_pitch_2 _returnvalue_yaw_2) (`KismetMathLibrary.BreakRotator` (`self.GetControlRotation`)))
  (:`Triggered`
    (`self.AddMovementInput` (`KismetMathLibrary.GetRightVector` (`KismetMathLibrary.MakeRotator` _returnvalue_roll_2 0.0 _returnvalue_yaw_2)) ActionValue_X)
    (`self.AddMovementInput` (`KismetMathLibrary.GetForwardVector` (`KismetMathLibrary.MakeRotator` 0.0 0.0 _returnvalue_yaw)) ActionValue_Y)))

(event `EnhancedInput|/Game/Skvt/Characters/Input/Actions/IA_Crouch`
  (params (ActionValue :type Boolean) (ElapsedSeconds :type "Float (double-precision)") (TriggeredSeconds :type "Float (double-precision)") (InputAction :type "InputAction Object Reference" :default "/Game/Skvt/Characters/Input/Actions/IA_Crouch.IA_Crouch"))
  (bind _charactermovement (`self.CharacterMovement`))
  (:`Triggered`
    (if (not (`self.bIsCrouched`))
      (`self.Crouch`)
      (set `CharacterMovementComponent.JumpZVelocity` 500.0 _charactermovement)
      (`self.OffsetCameraZ` 25.0)
      (bind (_direction _cameraarmlength _cameraz) (`Timeline|CrouchCameraAttributesTimeline` :!label _label)
        (:`Update`
          (set `SpringArmComponent.TargetArmLength` _cameraarmlength (`self.CameraBoom`))))
      (else
        (`self.UnCrouch`)
        (set `CharacterMovementComponent.JumpZVelocity` 580.0 _charactermovement)
        (`self.OffsetCameraZ` -25.0)
        (goto _label :!via `Reverse`)))))

(fn `CanJumpInternal`
  (returns (ReturnValue :type Boolean))
  (bind _charactermovement (`self.CharacterMovement`))
  (`/Engine/EditorBlueprintResources/StandardMacros.IsValid` _charactermovement
    (:`Is Valid`
      (if (`NavMovementInterface.IsFalling` _charactermovement)
        (return false)
        (else
          (return true))))
    (:`Is Not Valid`
      (return false))))

(fn `OffsetCameraZ`
  (params (Offset :type "Float (double-precision)"))
  (bind _cameraboom (`self.CameraBoom`))
  (bind (_returnvalue_x _returnvalue_y _returnvalue_z) (`KismetMathLibrary.BreakVector` (`SceneComponent.K2_GetComponentLocation` _cameraboom)))
  (`SceneComponent.K2_SetWorldLocation` _cameraboom (`KismetMathLibrary.MakeVector` _returnvalue_x _returnvalue_y (`KismetMathLibrary.FInterpTo_Constant` (+ _returnvalue_z Offset) _returnvalue_z (`GameplayStatics.GetWorldDeltaSeconds`) 7.0)) false false))

(fn `UserConstructionScript`)